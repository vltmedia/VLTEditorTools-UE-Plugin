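; BP_VLTP_LevelPlacementManager is a registry of spawned objects for the VLTPipe level creation tools.
; It stores each base object with its original object, path and category in SpawnedObjects, printing each addition.
; Helper functions rebuild the unique category list from those entries and return entries by category.
; Cleanup removes entries whose base object is still valid during iteration; construction and events are empty, and DOTHIS is a debug print.
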(event EventBeginPlay)

(event Collision|EventActorBeginOverlap
  (params (OtherActor :type Actor%20Object%20Reference)))

(event EventTick
  (params (DeltaSeconds :type Float%20%28single-precision%29)))

(fn ConstructionScript)

(fn AddNewSpawnedActor
  (params (BaseObject :type Actor%20Object%20Reference) (OriginalObject :type Actor%20Object%20Reference) (OriginalObjectPath :type String) (Category :type String))
  (Development|PrintString (Utilities|GetDisplayName BaseObject))
  (bind _returnvalue (Utilities|Array|Add (Variables|Default|GetSpawnedObjects) (Utilities|Struct|MakeStruct_VLTP_LevelObject BaseObject OriginalObject OriginalObjectPath Category)))
  (Development|PrintString (Utilities|String|ToString(Integer) _returnvalue)))

(fn UpdateCategories
  (bind _categories (Variables|Default|GetCategories))
  (Utilities|Array|Clear _categories)
  (for _array_element (Variables|Default|GetSpawnedObjects)
    (if (not (Utilities|Array|ContainsItem _categories (.category _array_element)))
      (Utilities|Array|Add _categories (.category _array_element)))))

(fn GetObjectsOfCategory
  (params (Category :type String))
  (bind _selectedbycategory_ (Variables|Default|GetSelectedByCategory_))
  (for _array_element (Variables|Default|GetSpawnedObjects)
    (if (Utilities|Enum|Equal(Enum) (.Category (Utilities|Struct|BreakStruct_VLTP_LevelObject _array_element)) Category)
      (Utilities|Array|Add _selectedbycategory_ _array_element)))
  (return _selectedbycategory_))

(fn CleanupSpawnedActors
  (bind _spawnedobjects (Variables|Default|GetSpawnedObjects))
  (for _array_element _spawnedobjects
    (Utilities|IsValid (.BaseObject (Utilities|Struct|BreakStruct_VLTP_LevelObject _array_element))
      (:Is%20Valid
        (Utilities|Array|RemoveItem _spawnedobjects _array_element)))))

(fn DOTHIS
  (Development|PrintString "Hello"))